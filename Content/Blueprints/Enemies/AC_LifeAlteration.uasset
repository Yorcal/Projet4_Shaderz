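; AC_LifeAlteration is an actor component that alters a BP_BaseEnemy's body material to reflect its life.
; On BeginPlay it caches the owning enemy and creates a dynamic material instance on slot 0 of its mesh.
; Externally triggered events drive the LerpAlpha scalar parameter: clamped Life/MaxLife while alive, a supplied Alpha when dead.
; Unconnected material setter nodes remain in the graph as a reference.
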(event Custom|UpdateRenderingWhenAlive
  (bind _enemy (Variables|Default|GetEnemy))
  (if (and (Utilities|IsValid (Variables|Default|GetEnemy)) (Utilities|IsValid (Variables|Default|GetMI_Body)))
    (Rendering|Material|SetScalarParameterValue (Variables|Default|GetMI_Body) "LerpAlpha" (Math|Float|Clamp(Float) (/ (Variables|/Game/Blueprints/Enemies/BP_BaseEnemy.BP_BaseEnemy_C|GetLife _enemy) (Variables|/Game/Blueprints/Enemies/BP_BaseEnemy.BP_BaseEnemy_C|GetMaxLife _enemy))) :!class /Script/Engine.MaterialInstanceDynamic)))

(event Custom|UpdateRenderingWhenDead
  (params (Alpha :type Float%20%28single-precision%29))
  (if (and (Utilities|IsValid (Variables|Default|GetEnemy)) (Utilities|IsValid (Variables|Default|GetMI_Body)))
    (Rendering|Material|SetScalarParameterValue (Variables|Default|GetMI_Body) "LerpAlpha" Alpha :!class /Script/Engine.MaterialInstanceDynamic)))

(event EventBeginPlay
  (bind _asbp_base_enemy (Utilities|Casting|CastToBP_BaseEnemy (Components|GetOwner)))
  (Variables|Default|SetEnemy _asbp_base_enemy)
  (CallFunction|UpdateMaterialInstance))

(fn UpdateMaterialInstance
  (bind _enemy (Variables|Default|GetEnemy))
  (bind _mesh (Variables|/Script/Engine.Character|GetMesh _enemy))
  (Utilities|IsValid _enemy
    (:Is%20Valid
      (bind _returnvalue (Rendering|Material|CreateDynamicMaterialInstance _mesh 0 (Rendering|Material|GetMaterial _mesh 0) "None" :!class /Script/Engine.PrimitiveComponent))
      (Variables|Default|SetMI_Body _returnvalue))))